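; Avalon Raft, a rideable ARK raft character with server-configurable stats and a switchable sail skin.
; On authority, BeginPlay applies GameMode INI options for speed, structure limits, health and weight; the server adds Buff_AvalonRaft then and on rider or possession changes.
; KnockRaft damage picks one of four directional knockback montages using dot products.
; A same-team multi-use entry toggles replicated SwitchTexture, whose OnRep swaps between vanilla and Avalon sail materials.
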(event Custom|SwapTexture
  (bind _self self)
  (bind _mesh (Variables|/Script/Engine.Character|GetMesh _self))
  ;[1 1 1] MUEntry that changes texture for sail
  (if (Variables|Default|GetSwitchTexture)
    (bind _returnvalue (Rendering|Material|CreateDynamicMaterialInstance "/Game/PrimalEarth/Items/Raft/Sail_Colorize_MIC.Sail_Colorize_MIC" :!class /Script/Engine.KismetMaterialLibrary))
    (Rendering|Material|SetMaterial _mesh 1 _returnvalue)
    (else
      (bind _returnvalue_2 (Rendering|Material|CreateDynamicMaterialInstance "/Game/Mods/AvalonRaft/MIC/AvalonRaftSail_Colorize_MIC.AvalonRaftSail_Colorize_MIC" :!class /Script/Engine.KismetMaterialLibrary))
      (Rendering|Material|SetMaterial _mesh 1 _returnvalue_2))))

(event Custom|DoPlayKnockAnimation
  (params (KnockDirectionIndex :type Integer))
  ;[1 1 1] Vanilla
  (if (not (Networking|IsDedicatedServer))
    (Class|PrimalCharacter|PlayAnimEx (Utilities|Array|Get(acopy) (Variables|Default|GetKnockbackAnims) KnockDirectionIndex) 1.0 "None" false false false false false 0.0 0.0)))

(event EventBPNotifySetRider
  (params (RiderSetting :type Shooter%20Character%20Object%20Reference))
  ;[1 1 1] Init
  ;[1 1 1] Add buff logic
  (if (Networking|IsServer)
    (Class|PrimalBuff|StaticAddBuff "/Game/Mods/AvalonRaft/BP/Buff_AvalonRaft.Buff_AvalonRaft_C" self 0 0 false)))

(event EventPossessed
  (params (NewController :type Controller%20Object%20Reference))
  ;[1 1 1] Init
  ;[1 1 1] Add buff logic
  (if (Networking|IsServer)
    (Class|PrimalBuff|StaticAddBuff "/Game/Mods/AvalonRaft/BP/Buff_AvalonRaft.Buff_AvalonRaft_C" self 0 0 false)))

(event EventBeginPlay
  (bind _returnvalue (Components|GetOwner))
  (bind _returnvalue_2 (Components|GetOwner))
  ;[1 1 1] Init
  (Utilities|FlowControl|Sequence
    (:then_0
      ;[1 1 1] Init ini-options
      (Utilities|FlowControl|Delay 0.2)
      (Networking|SwitchHasAuthority
        (:Authority
          (bind _asshootergamemode (Utilities|Casting|CastToShooterGameMode (Game|GetGameMode)))
          (Utilities|FlowControl|Sequence
            (:then_0
              ;[1 1 1] Ini for speed
              (bind _returnvalue_3 (Class|ShooterGameMode|GetFloatOptionIni _asshootergamemode "AvalonRaft" "RaftSpeed"))
              (if (>= _returnvalue_3 1.0)
                (if (<= _returnvalue_3 1e+03)
                  (Variables|Default|SetRaftSpeed _returnvalue_3)
                  (else
                    (Variables|Default|SetRaftSpeed 1.0 :!label _label)))
                (else
                  (goto _label)))
              (bind _returnvalue_4 (Class|PrimalCharacter|GetCharacterStatusComponent))
              (Class|PrimalCharacterStatusComponent|SetMaxStatusValue _returnvalue_4 "SpeedMultiplier" (* (Class|PrimalCharacterStatusComponent|BPGetMaxStatusValue _returnvalue_4 "SpeedMultiplier") (Variables|Default|GetRaftSpeed))))
            (:then_2
              ;[1 1 1] Ini for max structures
              (bind _returnvalue_5 (Class|ShooterGameMode|GetFloatOptionIni _asshootergamemode "AvalonRaft" "RaftMaxStructuresNum"))
              (if (<= _returnvalue_5 0.0)
                (Variables|Default|SetMaxSaddleStructuresNum 140)
                (else
                  (Variables|Default|SetMaxSaddleStructuresNum (Math|Float|Floor _returnvalue_5)))))
            (:then_3
              ;[1 1 1] Ini for structure height
              (bind _returnvalue_6 (Class|ShooterGameMode|GetFloatOptionIni _asshootergamemode "AvalonRaft" "RaftMaxStructuresHeight"))
              (if (<= _returnvalue_6 0.0)
                (Variables|Default|SetMaxSaddleStructuresHeight 2200)
                (else
                  (Variables|Default|SetMaxSaddleStructuresHeight (Math|Float|Floor _returnvalue_6)))))
            (:then_4
              ;[1 1 1] Ini for health
              (bind _returnvalue_7 (Class|ShooterGameMode|GetFloatOptionIni _asshootergamemode "AvalonRaft" "RaftHealth"))
              (if (<= _returnvalue_7 0.0)
                (bind _asprimaldinocharacter (Utilities|Casting|CastToPrimalDinoCharacter _returnvalue_2))
                (Class|PrimalCharacterStatusComponent|SetMaxStatusValue (Variables|/Script/ShooterGame.PrimalCharacter|GetMyCharacterStatusComponent _asprimaldinocharacter) "Health" 3.5e+04)
                (else
                  (bind _asprimaldinocharacter_2 (Utilities|Casting|CastToPrimalDinoCharacter _returnvalue_2))
                  (Class|PrimalCharacterStatusComponent|SetMaxStatusValue (Variables|/Script/ShooterGame.PrimalCharacter|GetMyCharacterStatusComponent _asprimaldinocharacter_2) "Health" _returnvalue_7))))
            (:then_5
              ;[1 1 1] Ini for weight
              (bind _returnvalue_8 (Class|ShooterGameMode|GetFloatOptionIni _asshootergamemode "AvalonRaft" "RaftMaxWeight"))
              (if (<= _returnvalue_8 0.0)
                (bind _asprimaldinocharacter_3 (Utilities|Casting|CastToPrimalDinoCharacter _returnvalue))
                (Class|PrimalCharacterStatusComponent|SetMaxStatusValue (Variables|/Script/ShooterGame.PrimalCharacter|GetMyCharacterStatusComponent _asprimaldinocharacter_3) "Weight" 3.6e+03)
                (else
                  (bind _asprimaldinocharacter_4 (Utilities|Casting|CastToPrimalDinoCharacter _returnvalue))
                  (Class|PrimalCharacterStatusComponent|SetMaxStatusValue (Variables|/Script/ShooterGame.PrimalCharacter|GetMyCharacterStatusComponent _asprimaldinocharacter_4) "Weight" _returnvalue_8))))))))
    (:then_1
      ;[1 1 1] Add buff logic
      (if (Networking|IsServer)
        (Class|PrimalBuff|StaticAddBuff "/Game/Mods/AvalonRaft/BP/Buff_AvalonRaft.Buff_AvalonRaft_C" self 0 0 false)))))

(fn ConstructionScript)

(fn ReceiveAnyDamage
  (params (Damage :type Float%20%28single-precision%29) (DamageType :type Damage%20Type%20Object%20Reference) (InstigatedBy :type Controller%20Object%20Reference) (DamageCauser :type Actor%20Object%20Reference))
  (bind _returnvalue (Transformation|GetActorLocation DamageCauser))
  (bind _returnvalue_2 (Transformation|GetActorForwardVector))
  (bind _returnvalue_3 (Transformation|GetActorRightVector))
  (bind _mesh (Variables|Character|GetMesh))
  (bind (_x _y) (Math|Vector|BreakVector _returnvalue_2))
  (bind (_x_2 _y_2) (Math|Vector|BreakVector _returnvalue_3))
  (bind _returnvalue_4 (Transformation|GetWorldLocation _mesh))
  (bind _returnvalue_5 (Math|Vector|MakeVector _x_2 _y_2 0.0))
  (bind _returnvalue_6 (Math|Vector|MakeVector _x _y 0.0))
  (bind _returnvalue_7 (- _returnvalue _returnvalue_4))
  (bind (_x_3 _y_3) (Math|Vector|BreakVector _returnvalue_7))
  (bind _returnvalue_8 (Math|Vector|Normalize _returnvalue_5))
  (bind _returnvalue_9 (Math|Vector|Normalize _returnvalue_6))
  (bind _returnvalue_10 (Math|Vector|MakeVector _x_3 _y_3 0.0))
  (bind _returnvalue_11 (Math|Vector|Normalize _returnvalue_10))
  (bind _returnvalue_12 (Math|Vector|DotProduct _returnvalue_11 _returnvalue_9))
  (bind _returnvalue_13 (Math|Vector|DotProduct _returnvalue_11 _returnvalue_8))
  (if (and (> Damage 0.0) (Networking|IsServer))
    (bind _asshooterdamagetypebp_base_c (Utilities|Casting|CastToShooterDamageTypeBP_Base DamageType))
    (if (Variables|/Game/PrimalEarth/CoreBlueprints/DamageTypes/ShooterDamageTypeBP_Base.ShooterDamageTypeBP_Base_C|GetbKnockRaft _asshooterdamagetypebp_base_c)
      (LocalVariables|SetRetVal 0)
      (if (and (>= _returnvalue_12 0.7) (Math|Float|InRange(Float) _returnvalue_13 -0.71 0.71))
        (LocalVariables|SetRetVal 0)
        (CallFunction|DoPlayKnockAnimation (LocalVariables|GetRetVal) :!label _label)
        (elif (and (>= _returnvalue_13 0.71) (Math|Float|InRange(Float) _returnvalue_12 -0.71 0.71))
          (LocalVariables|SetRetVal 1)
          (goto _label)
          (elif (and (>= -0.71 _returnvalue_12) (Math|Float|InRange(Float) _returnvalue_13 -0.71 0.71))
            (LocalVariables|SetRetVal 2)
            (goto _label)
            (elif (and (>= -0.71 _returnvalue_13) (Math|Float|InRange(Float) _returnvalue_12 -0.71 0.71))
              (LocalVariables|SetRetVal 3)
              (goto _label))))))))

(fn BPTryMultiUse
  (params (ForPC :type Player%20Controller%20Object%20Reference) (UseIndex :type Integer))
  (Utilities|FlowControl|Sequence
    (:then_0
      (switch int UseIndex
        (:2476
          (Variables|Default|SetSwitchTexture (not (Variables|Default|GetSwitchTexture)) true))))
    (:then_1
      (return true))))

(fn BPGetMultiUseEntries
  (params (ForPC :type Player%20Controller%20Object%20Reference) (MultiUseEntries :type Array%20of%20Multi%20Use%20Entry%20Structures))
  (Variables|Default|SetMUEntry MultiUseEntries)
  (if (== (Variables|/Script/Engine.Actor|GetTargetingTeam ForPC) (Variables|Default|GetTargetingTeam))
    (Utilities|Array|Add MultiUseEntries (Utilities|Struct|MakeMultiUseEntry 0 (Utilities|String|SelectString "Avalon Sail" "Vanilla Sail" (Variables|Default|GetSwitchTexture)) 2476 -1 false false false false false false false false false true false false false 0 "(B=175,G=175,R=175,A=255)" (Math|Conversions|ToColor(LinearColor) "(R=255.000000,G=0.000000,B=0.000000,A=1.000000)"))))
  (return MultiUseEntries))

(fn OnRepSwitchTexture
  (CallFunction|SwapTexture))